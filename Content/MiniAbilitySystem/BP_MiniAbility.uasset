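; BP_MiniAbility is the base ability object for the Mini Ability System, with empty lifecycle events for initialization, activation, tick, activated tags, messages and ending.
; CanActivateAbility returns true by default.
; Helpers append or remove tags in ActivationTags and expose the ability parameter and owning MiniAbilityManagerComponent.
; EndAbility delegates to that manager's EndAbilityObject, passing itself and the cancelled flag.
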(event Custom|ActivateAbility)

(event Custom|OnEndAbility
  (params (InCancelled :type Boolean)))

(event Custom|OnMessageReceived
  (params (InMessage :type String)))

(event Custom|Initialize)

(event Custom|OnActivatedTags
  (params (InTagContainer :type Gameplay%20Tag%20Container%20Structure) (InAbilityParam :type BPI%20Mini%20Ability%20Param%20Interface)))

(event Custom|Tick
  (params (DeltaSeconds :type Float%20%28single-precision%29)))

(fn CanActivateAbility
  (return true))

(fn AddAbilityTags
  (params (InTags :type Gameplay%20Tag%20Container%20Structure))
  (GameplayTags|AppendGameplayTagContainers (Variables|MiniAbility|GetActivationTags) InTags))

(fn RemoveAbilityTag
  (params (InTag :type Gameplay%20Tag%20Structure))
  (bind _returnvalue (GameplayTags|RemoveGameplayTag (Variables|MiniAbility|GetActivationTags) InTag :!class /Script/GameplayTags.BlueprintGameplayTagLibrary))
  (return _returnvalue))

(fn GetAbilityManager
  (return (Variables|Private|GetMiniAbilityManagerComponent)))

(fn GetAbilityParam
  (return (Variables|Private|GetAbilityParam)))

(fn EndAbility
  (params (InCancelled :type Boolean))
  (Default|EndAbilityObject (MiniAbility|GetAbilityManager) self InCancelled))