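; Actor component that runs a lightweight, tag-driven ability system, similar in concept to GAS.
; It seeds ability classes at BeginPlay, activates them by tag as constructed objects, and ticks every active object.
; Activation checks block and required tags against running abilities, then cancels those matching the new ability's cancel tags.
; Tag queries also route messages and remove classes, while ending an ability here only drops it from the active list.
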(event EventBeginPlay
  (Variables|Private|SetAbilityClasses (Variables|MiniAbilityManager|GetInitialAbilityClasses)))

(event EventTick
  (params (DeltaSeconds :type Float%20%28single-precision%29))
  (for _array_element (Variables|Private|GetAbilityObjects)
    (Default|Tick _array_element (Utilities|Time|GetWorldDeltaSeconds))))

(fn AddAbilityClasses
  (params (InAddClasses :type Array%20of%20BP%20Mini%20Ability%20Class%20References))
  (for _array_element InAddClasses
    (Utilities|Array|AddUnique (Variables|Private|GetAbilityClasses) _array_element)))

(fn RemoveAbilityClasses
  (params (InRemoveClasses :type Array%20of%20BP%20Mini%20Ability%20Class%20References))
  (for _array_element InRemoveClasses
    (bind _returnvalue (Utilities|Array|RemoveItem (Variables|Private|GetAbilityClasses) _array_element))
    (if _returnvalue
      (LocalVariables|SetbResult true)))
  (return (LocalVariables|GetbResult)))

(fn ActivateAbilityClass
  (params (InAbilityClass :type BP%20Mini%20Ability%20Class%20Reference) (InAbilityParam :type BPI%20Mini%20Ability%20Param%20Interface))
  (LocalVariables|SetAbilityClass InAbilityClass)
  (LocalVariables|SetAbilityParam InAbilityParam)
  (if (not (Private|IsAbilityClassBlocked (LocalVariables|GetAbilityClass)))
    (Utilities|Casting|CastToBPI_MiniAbilityParam (LocalVariables|GetAbilityParam)
      (:then
        (bind _returnvalue (Game|ConstructObjectfromClass (LocalVariables|GetAbilityClass) self self (LocalVariables|GetAbilityParam)))
        (LocalVariables|SetAbilityObject _returnvalue))
      (:CastFailed
        (bind _returnvalue_2 (Game|ConstructObjectfromClass (LocalVariables|GetAbilityClass) self self 0))
        (LocalVariables|SetAbilityObject _returnvalue_2)))
    (Default|Initialize (LocalVariables|GetAbilityObject))
    (if (Default|CanActivateAbility (LocalVariables|GetAbilityObject))
      (LocalVariables|SetCancelTags (Variables|/Game/MiniAbilitySystem/BP_MiniAbility.BP_MiniAbility_C|GetCancelAbilitiesWithTag (LocalVariables|GetAbilityObject)))
      (if (== (GameplayTags|GetNumGameplayTagsinContainer (LocalVariables|GetCancelTags)) 0)
        _
        (else
          (MiniAbilityManager|EndAbilityObjectswithTags (LocalVariables|GetCancelTags) true)))
      (Utilities|Array|Add (Variables|Private|GetAbilityObjects) (LocalVariables|GetAbilityObject))
      (Default|AddAbilityTags (LocalVariables|GetAbilityObject) (Variables|/Game/MiniAbilitySystem/BP_MiniAbility.BP_MiniAbility_C|GetActivationOwnedTags (LocalVariables|GetAbilityObject)))
      (Default|ActivateAbility (LocalVariables|GetAbilityObject))
      (return true)
      (else
        (return false)))
    (else
      (return false))))

(fn GetBlockTagsOfAbilityObjects
  (for _array_element (Variables|Private|GetAbilityObjects)
    (LocalVariables|SetAbilityObject _array_element)
    (GameplayTags|AppendGameplayTagContainers (LocalVariables|GetBlockTags) (Variables|/Game/MiniAbilitySystem/BP_MiniAbility.BP_MiniAbility_C|GetBlockAbilitiesWithTag (LocalVariables|GetAbilityObject))))
  (return (LocalVariables|GetBlockTags)))

(fn GetActivationTagsOfAbilityObjects
  (for _array_element (Variables|Private|GetAbilityObjects)
    (LocalVariables|SetAbilityObject _array_element)
    (GameplayTags|AppendGameplayTagContainers (LocalVariables|GetActivationTags) (Variables|/Game/MiniAbilitySystem/BP_MiniAbility.BP_MiniAbility_C|GetActivationTags (LocalVariables|GetAbilityObject))))
  (return (LocalVariables|GetActivationTags)))

(fn IsAbilityClassBlocked
  (params (InAbilityClass :type BP%20Mini%20Ability%20Class%20Reference))
  (bind (_activationtags _cancelabilitieswithtag _blockabilitieswithtag _activationownedtags _activationblockedtags _activationrequiredtags) (Utilities|GetClassDefaults InAbilityClass))
  (return (Math|Boolean|ORBoolean (GameplayTags|HasAnyTags _activationtags (Private|GetBlockTagsOfAbilityObjects)) (GameplayTags|HasAnyTags _activationownedtags (Private|GetBlockTagsOfAbilityObjects)) (GameplayTags|HasAnyTags (Private|GetActivationTagsOfAbilityObjects) _activationblockedtags) (not (GameplayTags|HasAllTags (Private|GetActivationTagsOfAbilityObjects) _activationrequiredtags)))))

(fn EndAbilityObjectswithTags
  (params (InTags :type Gameplay%20Tag%20Container%20Structure) (InCancelled :type Boolean))
  (LocalVariables|SetTags InTags)
  (LocalVariables|SetbCancelled InCancelled)
  (for _array_element (Private|GetAbilityObjectswithTags (LocalVariables|GetTags))
    (bind _outvalue (MiniAbilityManager|EndAbilityObject _array_element (LocalVariables|GetbCancelled)))
    (if _outvalue
      (LocalVariables|SetbResult true)))
  (return (LocalVariables|GetbResult)))

(fn GetAbilityObjectswithTags
  (params (InTags :type Gameplay%20Tag%20Container%20Structure))
  (LocalVariables|SetTags InTags)
  (for _array_element (Variables|Private|GetAbilityObjects)
    (LocalVariables|SetAbilityObject _array_element)
    (if (GameplayTags|HasAllTags (Variables|/Game/MiniAbilitySystem/BP_MiniAbility.BP_MiniAbility_C|GetActivationTags (LocalVariables|GetAbilityObject)) (LocalVariables|GetTags))
      (Utilities|Array|Add (LocalVariables|GetMiniAbilityObjectsWithTags) (LocalVariables|GetAbilityObject))))
  (return (LocalVariables|GetMiniAbilityObjectsWithTags)))

(fn SendMessagewithTags
  (params (InTags :type Gameplay%20Tag%20Container%20Structure) (InMessage :type String))
  (LocalVariables|SetTags InTags)
  (LocalVariables|SetMessage InMessage)
  (for _array_element (Private|GetAbilityObjectswithTags (LocalVariables|GetTags))
    (Default|OnMessageReceived _array_element (LocalVariables|GetMessage))
    (LocalVariables|SetbResult true))
  (return (LocalVariables|GetbResult)))

(fn EndAbilityObject
  (params (InAbilityObject :type BP%20Mini%20Ability%20Object%20Reference) (InCancelled :type Boolean))
  (LocalVariables|SetAbilityObject InAbilityObject)
  (LocalVariables|SetbCancelled InCancelled)
  (if (Utilities|Array|ContainsItem (Variables|Private|GetAbilityObjects) (LocalVariables|GetAbilityObject))
    (bind _returnvalue (Utilities|Array|RemoveItem (Variables|Private|GetAbilityObjects) (LocalVariables|GetAbilityObject)))
    (return _returnvalue)
    (else
      (return false))))

(fn DebugPrint
  (for _array_element (Variables|Private|GetAbilityObjects)
    (LocalVariables|SetAbility _array_element)
    (Development|PrintString (GameplayTags|GetDebugStringfromGameplayTagContainer (Variables|/Game/MiniAbilitySystem/BP_MiniAbility.BP_MiniAbility_C|GetActivationTags (LocalVariables|GetAbility))))))

(fn ActivateAbilityClasseswithTags
  (params (InActivateTags :type Gameplay%20Tag%20Container%20Structure) (InAbilityParam :type BPI%20Mini%20Ability%20Param%20Interface))
  (LocalVariables|SetActivateTags InActivateTags)
  (LocalVariables|SetAbilityParam InAbilityParam)
  (for _array_element (Variables|Private|GetAbilityClasses)
    (LocalVariables|SetAbilityClass _array_element)
    (LocalVariables|SetAbilityTags (.ActivationTags (Utilities|GetClassDefaults (LocalVariables|GetAbilityClass))))
    (if (GameplayTags|HasAllTags (LocalVariables|GetAbilityTags) (LocalVariables|GetActivateTags))
      (bind _outvalue (MiniAbilityManager|ActivateAbilityClass (LocalVariables|GetAbilityClass) (LocalVariables|GetAbilityParam)))
      (if _outvalue
        (LocalVariables|SetbResult true))))
  (for _array_element_2 (Variables|Private|GetAbilityObjects)
    (Default|OnActivatedTags _array_element_2 (LocalVariables|GetActivateTags) (LocalVariables|GetAbilityParam)))
  (return (LocalVariables|GetbResult)))

(fn HasAbilityObjectsTags
  (params (InTags :type Gameplay%20Tag%20Container%20Structure))
  (LocalVariables|SetTags InTags)
  (for _array_element (Variables|Private|GetAbilityObjects)
    (LocalVariables|SetAbilityObjectTags (Variables|/Game/MiniAbilitySystem/BP_MiniAbility.BP_MiniAbility_C|GetActivationTags _array_element))
    (if (GameplayTags|HasAllTags (LocalVariables|GetAbilityObjectTags) (LocalVariables|GetTags))
      (return true)))
  (return false))

(fn RemoveAbilityClasseswithTags
  (params (InTags :type Gameplay%20Tag%20Container%20Structure))
  (LocalVariables|SetTags InTags)
  (for _array_element (Variables|Private|GetAbilityClasses)
    (LocalVariables|SetCheckAbilityClass _array_element)
    (LocalVariables|SetActivationTags (.ActivationTags (Utilities|GetClassDefaults (LocalVariables|GetCheckAbilityClass))))
    (GameplayTags|AppendGameplayTagContainers (LocalVariables|GetActivationTags) (.ActivationOwnedTags (Utilities|GetClassDefaults (LocalVariables|GetCheckAbilityClass))))
    (if (GameplayTags|HasAllTags (LocalVariables|GetActivationTags) (LocalVariables|GetTags))
      (Utilities|Array|Add (LocalVariables|GetRemoveAbilityClassList) (LocalVariables|GetCheckAbilityClass))))
  (bind _outvalue (MiniAbilityManager|RemoveAbilityClasses (LocalVariables|GetRemoveAbilityClassList)))
  (return _outvalue))